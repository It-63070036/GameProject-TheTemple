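; BP_PowerCell is a collectible power cell that stays collected through the game instance's SaveGameState.
; On overlap it sets itself as RefPowerCell on BP_FirstPersonCharacter, exposing a PickUp event that registers its ActorID via CollectPowerCellSystem.
; Shortly after BeginPlay it asks SaveGameState whether that ActorID was already picked up and destroys itself if so.
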(event `self.Collision.OnComponentBeginOverlap`
  (params (OverlappedComponent :type "PrimitiveComponent Object Reference") (OtherActor :type "Actor Object Reference") (OtherComp :type "PrimitiveComponent Object Reference") (OtherBodyIndex :type Integer) (bFromSweep :type Boolean) (SweepResult :type "HitResult Structure (by ref)"))
  (bind _asbp_first_person_character (cast `/Game/Develop/Blueprints/BP_FirstPersonCharacter` OtherActor))
  (set `/Game/Develop/Blueprints/BP_FirstPersonCharacter.RefPowerCell` self _asbp_first_person_character))

(event `self.ReceiveBeginPlay`
  (`KismetSystemLibrary.Delay` 0.2)
  (bind _assave_game_state (cast `/Game/Develop/Blueprints/GameInstance/SaveGameState` (`GameplayStatics.GetGameInstance`)))
  (bind _picked_up (`/Game/Develop/Blueprints/GameInstance/SaveGameState.CheckIfAlreadyPickup` _assave_game_state (`self.ActorID`)))
  (if _picked_up
    (`self.K2_DestroyActor`)))

(event `PickUp`
  (bind _assave_game_state (cast `/Game/Develop/Blueprints/GameInstance/SaveGameState` (`GameplayStatics.GetGameInstance`)))
  (`/Game/Develop/Blueprints/GameInstance/SaveGameState.CollectPowerCellSystem` _assave_game_state (`self.ActorID`)))

(fn `UserConstructionScript`)