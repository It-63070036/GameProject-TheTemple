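; Laser generator actor that, while holding a power cell, fires a bouncing beam to activate goal spheres.
; Each Tick it line-traces from its Arrow, continuing along the hit normal off BPI_Reflective actors, and ends the current sphere's activation when none is hit.
; Beam segments reuse static mesh actors spawned at BeginPlay, stretched between trace points or hidden.
; Its collision box registers the generator on the overlapping first-person character.
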(event `self.ReceiveBeginPlay`
  ;[1 0.6942 0.3153] Spawn Laser Mesh
  (for _ (range (+ (`self.BounceAmount`) 1))
    (bind _returnvalue (`|SpawnActorFromClass` "/Script/Engine.StaticMeshActor" (`SceneComponent.K2_GetComponentToWorld` (`self.DefaultSceneRoot`)) "Undefined" "OverrideRootScale" null null))
    (`StaticMeshComponent.SetStaticMesh` (`StaticMeshActor.StaticMeshComponent` _returnvalue) "/Game/Develop/Mesh/SM_LaserMesh.SM_LaserMesh")
    (`StaticMeshActor.SetMobility` _returnvalue "Movable")
    (`KismetArrayLibrary.Array_Add` (`self.LaserMeshes`) _returnvalue)))

(event `self.ReceiveTick`
  (params (DeltaSeconds :type "Float (single-precision)"))
  (bind _arrow (`self.Arrow`))
  (bind _currentgoalsphere (`self.CurrentGoalSphere`))
  (bind (_bblockinghit _binitialoverlap _time _distance _location _impactpoint _normal) (`GameplayStatics.BreakHitResult` (`self.PreviousHit`)))
  ;[0.6045 0.5568 1] Check if Player have Power Cell
  (if (`self.HavePowerCell?`)
    ;[0.3065 1 0.3381] Shooting and Bouncing Laser
    (set `self.IsActivating?` false)
    (set `self.PreviousHit` (struct))
    (`self.BounceLaser` (`SceneComponent.K2_GetComponentLocation` _arrow) (`SceneComponent.GetForwardVector` _arrow))
    (`self.CheckIfHittingGoal`)
    (for _index (range 1 (+ (`self.BounceAmount`) 1))
      (if (and (`self.PreviousReturn`) (`KismetSystemLibrary.DoesImplementInterface` (`.HitActor` (`GameplayStatics.BreakHitResult` (`self.PreviousHit`))) "/Game/Develop/Blueprints/BPI_Reflective.BPI_Reflective_C"))
        (`self.BounceLaser` _location _normal _index)
        (`self.CheckIfHittingGoal`)
        (else
          (`self.HideLaserMesh` _index))))
    ;[1 0.3224 0.3124] Check if we are activating a goal sphere, Then end activation of current goal shpere
    (if (not (`self.IsActivating?`))
      (`/Engine/EditorBlueprintResources/StandardMacros.IsValid` _currentgoalsphere
        (:`Is Valid`
          (`/Game/Develop/Blueprints/BP_GoalSphere.EndActivation` _currentgoalsphere)
          (set `self.CurrentGoalSphere` null))))))

(event `self.CollisionBox.OnComponentBeginOverlap`
  (params (OverlappedComponent :type "PrimitiveComponent Object Reference") (OtherActor :type "Actor Object Reference") (OtherComp :type "PrimitiveComponent Object Reference") (OtherBodyIndex :type Integer) (bFromSweep :type Boolean) (SweepResult :type "HitResult Structure (by ref)"))
  ;[1 0.788 0.3209] Set Laser Generator Overlap Target
  (bind _asbp_first_person_character (cast `/Game/Develop/Blueprints/BP_FirstPersonCharacter` OtherActor))
  (set `/Game/Develop/Blueprints/BP_FirstPersonCharacter.OverLapLaserGenerator` self _asbp_first_person_character))

(fn `AddLaserMesh`
  (params (`Start Location` :type "Vector Structure") (`End Location` :type "Vector Structure") (Index :type Integer))
  (bind _output (`|GetArrayItem` (`self.LaserMeshes`) Index))
  (bind _staticmeshcomponent (`StaticMeshActor.StaticMeshComponent` _output))
  (`SceneComponent.K2_SetWorldLocationAndRotation` _staticmeshcomponent `Start Location` (`KismetMathLibrary.FindLookAtRotation` `Start Location` `End Location`) false false)
  (`SceneComponent.SetRelativeScale3D` _staticmeshcomponent (`KismetMathLibrary.MakeVector` (/ (`KismetMathLibrary.Vector_Distance` `End Location` `Start Location`) 10.0) 1.0 1.0))
  (`self.SetActorHiddenInGame` _output false))

(fn `BounceLaser`
  (params (StartLocation :type "Vector Structure") (Direction :type "Vector Structure") (Index :type Integer))
  (bind _index (`local.Index`))
  (bind _returnvalue (+ StartLocation (* Direction 15000.0)))
  (bind (_outhit _returnvalue_2) (`KismetSystemLibrary.LineTraceSingle` StartLocation _returnvalue "TraceTypeQuery1" false (`|MakeArray` (`.HitActor` (`GameplayStatics.BreakHitResult` (`self.PreviousHit`))))))
  (set `self.PreviousHit` _outhit)
  (bind _output_get (set `self.PreviousReturn` _returnvalue_2))
  (if _output_get
    (bind (_bblockinghit _binitialoverlap _time _distance _location _impactpoint _normal _impactnormal _physmat _hitactor _hitcomponent _hitbonename _bonename _hititem _elementindex _faceindex _tracestart) (`GameplayStatics.BreakHitResult` _outhit))
    (`self.AddLaserMesh` _tracestart _location _index)
    (else
      (`self.AddLaserMesh` _tracestart _returnvalue _index))))

(fn `CheckIfHittingGoal`
  (bind _asbp_goal_sphere (cast `/Game/Develop/Blueprints/BP_GoalSphere` (`.HitActor` (`GameplayStatics.BreakHitResult` (`self.PreviousHit`)))))
  (`/Game/Develop/Blueprints/BP_GoalSphere.StartActivation` _asbp_goal_sphere)
  (set `self.PreviousReturn` false)
  (set `self.CurrentGoalSphere` _asbp_goal_sphere)
  (set `self.IsActivating?` true))

(fn `HideLaserMesh`
  (params (Index :type Integer))
  (`self.SetActorHiddenInGame` (`|GetArrayItem` (`self.LaserMeshes`) Index) true))

(fn `UserConstructionScript`)