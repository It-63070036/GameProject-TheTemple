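; Activatable wall that destroys whatever object the first-person character is holding when the character overlaps its cube.
; Activate switches the destruction off and Deactivate switches it back on, each flipping a disable flag after a short delay.
; The cube's begin-overlap checks that flag, prints its state for debugging, and, when enabled, calls DestroyHeldObject on the overlapping character.
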(event `/Game/Develop/Blueprints/BPI_Activatable.Activate`
  (`KismetSystemLibrary.Delay` 1.0)
  (set `self.IsDestroyDisabled` true))

(event `/Game/Develop/Blueprints/BPI_Activatable.Deactivate`
  (`KismetSystemLibrary.Delay` 1.0)
  (set `self.IsDestroyDisabled` false))

(event `self.Cube.OnComponentBeginOverlap`
  (params (OverlappedComponent :type "PrimitiveComponent Object Reference") (OtherActor :type "Actor Object Reference") (OtherComp :type "PrimitiveComponent Object Reference") (OtherBodyIndex :type Integer) (bFromSweep :type Boolean) (SweepResult :type "HitResult Structure (by ref)"))
  (if (`self.IsDestroyDisabled`)
    (`KismetSystemLibrary.PrintString` "Disabled")
    (else
      (`KismetSystemLibrary.PrintString` "Not Disabled")
      (bind _asbp_first_person_character (cast `/Game/Develop/Blueprints/BP_FirstPersonCharacter` OtherActor))
      (`/Game/Develop/Blueprints/BP_FirstPersonCharacter.DestroyHeldObject` _asbp_first_person_character))))

(fn `UserConstructionScript`)