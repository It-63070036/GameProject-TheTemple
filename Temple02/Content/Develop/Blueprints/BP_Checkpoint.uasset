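; BP_Checkpoint is a checkpoint actor that sets the respawn point and saves progress when the player enters it.
; When BP_FirstPersonCharacter overlaps the Boundary, it builds a transform from the Cube's location and the character capsule's rotation and scale.
; That transform becomes the game mode's SpawnLocation, then the first player controller runs SaveGame, with debug prints confirming each step.
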(event `self.Boundary.OnComponentBeginOverlap`
  (params (OverlappedComponent :type "PrimitiveComponent Object Reference") (OtherActor :type "Actor Object Reference") (OtherComp :type "PrimitiveComponent Object Reference") (OtherBodyIndex :type Integer) (bFromSweep :type Boolean) (SweepResult :type "HitResult Structure (by ref)"))
  (bind _asbp_first_person_character (cast `/Game/Develop/Blueprints/BP_FirstPersonCharacter` OtherActor))
  (bind (_returnvalue_location _returnvalue_rotation _returnvalue_scale) (`KismetMathLibrary.BreakTransform` (`SceneComponent.K2_GetComponentToWorld` (`Character.CapsuleComponent` _asbp_first_person_character))))
  (set `self.LastLocation` (`KismetMathLibrary.MakeTransform` (`SceneComponent.K2_GetComponentLocation` (`self.Cube`)) _returnvalue_rotation _returnvalue_scale))
  (bind _asbp_first_person_game_mode (cast `/Game/Develop/Blueprints/BP_FirstPersonGameMode` (`GameplayStatics.GetGameMode`)))
  (`|ExecutionSequence`
    (:`then_0`
      (set `/Game/Develop/Blueprints/BP_FirstPersonGameMode.SpawnLocation` (`self.LastLocation`) _asbp_first_person_game_mode)
      (`KismetSystemLibrary.PrintString` "SpawnLocation Set"))
    (:`then_1`
      (bind _asbp_first_person_controller (cast `/Game/Develop/Blueprints/BP_FirstPersonController` (`GameplayStatics.GetPlayerController` 0)))
      (`/Game/Develop/Blueprints/BP_FirstPersonController.SaveGame` _asbp_first_person_controller)
      (`KismetSystemLibrary.PrintString` "Check Point Set"))))

(fn `UserConstructionScript`)