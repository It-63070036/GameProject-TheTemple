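; BP_Activatable_StoppingWall is an activatable wall that can block lasers.
; Activate turns off the cube's collision after a short delay, and Deactivate restores its LaserBlock collision profile the same way.
; LaserHitGoal destroys the actor after a delay, while LasernotHitGoal spawns a new copy at the transform saved on BeginPlay, without destroying the current one.
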(event `/Game/Develop/Blueprints/BPI_Activatable.Activate`
  (`KismetSystemLibrary.Delay` 0.2)
  (`PrimitiveComponent.SetCollisionEnabled` (`self.Cube`) "NoCollision"))

(event `/Game/Develop/Blueprints/BPI_Activatable.Deactivate`
  (`KismetSystemLibrary.Delay` 0.2)
  (`PrimitiveComponent.SetCollisionProfileName` (`self.Cube`) "LaserBlock" true))

(event `self.ReceiveBeginPlay`
  (set `self.RespawnLocation` (`SceneComponent.K2_GetComponentToWorld` (`self.DefaultSceneRoot`))))

(event `LaserHitGoal`
  (`KismetSystemLibrary.Delay` 1.0)
  (`self.K2_DestroyActor` self))

(event `LasernotHitGoal`
  (`KismetSystemLibrary.Delay` 1.0)
  (`|SpawnActorFromClass` "BP_Activatable_StoppingWall_C" (`self.RespawnLocation`) "AlwaysSpawn" "OverrideRootScale" null null))

(fn `UserConstructionScript`)