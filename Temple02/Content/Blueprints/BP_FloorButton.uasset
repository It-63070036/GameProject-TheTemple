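; Floor pressure button that activates linked objects while the first-person character or a physics-simulating component rests on it.
; Box overlap plays or reverses a timeline that moves the cylinder on Z.
; It sends activate and deactivate messages to ActivateObjects entries implementing BPI_Activatable.
; Release requires AreThereAnyobjOnTopOfButton, which, despite its name, returns true when no character or physics object remains.
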(event `DownAnimation`
  (bind (_direction _zoffset) (`Timeline|ButtonDown` :!label _label)
    (:`Update`
      (`SceneComponent.K2_SetRelativeLocation` (`self. Cylinder1`) (`KismetMathLibrary.MakeVector` 0.0 0.0 _zoffset) false false))))

(event `UpAnimation`
  (goto _label :!via `Reverse`))

(event `self.Box.OnComponentBeginOverlap`
  (params (OverlappedComponent :type "PrimitiveComponent Object Reference") (OtherActor :type "Actor Object Reference") (OtherComp :type "PrimitiveComponent Object Reference") (OtherBodyIndex :type Integer) (bFromSweep :type Boolean) (SweepResult :type "HitResult Structure (by ref)"))
  (if (or (== (`GameplayStatics.GetObjectClass` OtherActor) "/Game/Blueprints/BP_FirstPersonCharacter.BP_FirstPersonCharacter_C") (`SceneComponent.IsSimulatingPhysics` OtherComp "None"))
    (`self.DownAnimation`)
    (for _array_element (`self.ActivateObjects`)
      (if (`KismetSystemLibrary.DoesImplementInterface` _array_element "/Game/Blueprints/BPI_Activatable.BPI_Activatable_C")
        (message `/Game/Blueprints/BPI_Activatable.Activate` _array_element)))))

(event `self.Box.OnComponentEndOverlap`
  (params (OverlappedComponent :type "PrimitiveComponent Object Reference") (OtherActor :type "Actor Object Reference") (OtherComp :type "PrimitiveComponent Object Reference") (OtherBodyIndex :type Integer))
  (if (and (or (== (`GameplayStatics.GetObjectClass` OtherActor) "/Game/Blueprints/BP_FirstPersonCharacter.BP_FirstPersonCharacter_C") (`SceneComponent.IsSimulatingPhysics` OtherComp "None")) (`self.AreThereAnyobjOnTopOfButton`))
    (`self.UpAnimation`)
    (for _array_element (`self.ActivateObjects`)
      (if (`KismetSystemLibrary.DoesImplementInterface` _array_element "/Game/Blueprints/BPI_Activatable.BPI_Activatable_C")
        (message `/Game/Blueprints/BPI_Activatable.Deactivate` _array_element)))))

(fn `AreThereAnyobjOnTopOfButton`
  (returns (Return :type Boolean))
  (locals (IsObjOnButton :type Boolean))
  (for _array_element (`PrimitiveComponent.GetOverlappingComponents` (`self.Box`))
    (if (`SceneComponent.IsSimulatingPhysics` _array_element "None")
      (set `local.IsObjOnButton` true)))
  (return (and (not (`local.IsObjOnButton`)) (== (`KismetArrayLibrary.Array_Length` (`PrimitiveComponent.GetOverlappingActors` (`self.Box`) "/Game/Blueprints/BP_FirstPersonCharacter.BP_FirstPersonCharacter_C")) 0))))

(fn `UserConstructionScript`)