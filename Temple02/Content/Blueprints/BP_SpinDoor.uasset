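; BP_SpinDoor is a door that swings open on Activate and back on Deactivate.
; The DoorOpen timeline, with a configurable play rate, lerps the Cylinder's relative yaw from zero to the Arrow component's yaw, so the arrow defines the open angle.
; Activation first runs a sphere trace around the Cube to wake nearby physics-simulating bodies before the door moves.
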(event `self.ReceiveBeginPlay`
  (`TimelineComponent.SetPlayRate` (`self.DoorOpen`) (`self.PlayRate`)))

(event `/Game/Blueprints/BPI_Activatable.Activate`
  (bind (_relativerotation_roll _relativerotation_pitch _relativerotation_yaw) (`KismetMathLibrary.BreakRotator` (`SceneComponent.RelativeRotation` (`self.Arrow`))))
  (`self.WakeNearByObject`)
  (bind (_direction _amount) (`Timeline|DoorOpen` :!label _label)
    (:`Update`
      (`SceneComponent.K2_SetRelativeRotation` (`self.Cylinder`) (`KismetMathLibrary.MakeRotator` 0.0 0.0 (`KismetMathLibrary.Lerp` 0.0 _relativerotation_yaw _amount)) false false))))

(event `/Game/Blueprints/BPI_Activatable.Deactivate`
  (goto _label :!via `Reverse`))

(fn `UserConstructionScript`)

(fn `WakeNearByObject`
  (bind _returnvalue (`SceneComponent.K2_GetComponentLocation` (`self.Cube`)))
  (bind _outhits (`KismetSystemLibrary.SphereTraceMulti` _returnvalue _returnvalue 400.0 "TraceTypeQuery1"))
  (for _array_element _outhits
    (bind (_bblockinghit _binitialoverlap _time _distance _location _impactpoint _normal _impactnormal _physmat _hitactor _hitcomponent) (`GameplayStatics.BreakHitResult` _array_element))
    (if (`SceneComponent.IsSimulatingPhysics` _hitcomponent "None")
      (`PrimitiveComponent.WakeAllRigidBodies` _hitcomponent))))