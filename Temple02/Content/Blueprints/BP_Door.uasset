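; BP_Door is a sliding door that opens on Activate and closes on Deactivate.
; The DoorOpen timeline plays forward or in reverse at the PlayRate set on BeginPlay.
; Each update sets the Cube's relative location to a lerp from zero to DistanceAmount along the Arrow component's forward vector, so the arrow defines the slide direction.
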(event `self.ReceiveBeginPlay`
  (`TimelineComponent.SetPlayRate` (`self.DoorOpen`) (`self.PlayRate`)))

(event `/Game/Blueprints/BPI_Activatable.Activate`
  (bind (_direction _amount) (`Timeline|DoorOpen` :!label _label)
    (:`Update`
      (`SceneComponent.K2_SetRelativeLocation` (`self.Cube`) (* (`KismetMathLibrary.Lerp` 0.0 (`self.DistanceAmount`) _amount) (`SceneComponent.GetForwardVector` (`self.Arrow`))) false false))))

(event `/Game/Blueprints/BPI_Activatable.Deactivate`
  (goto _label :!via `Reverse`))

(fn `UserConstructionScript`)